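; Container trailer that mirrors the player truck's blinker, side and brake lights and lets the truck know when it is in attach range.
; While ActiveLight is set, Tick polls the player's Truck_BP flags, with a timeline pulsing the blinkers.
; The lights are dynamic material instances created in the construction script, plus two brake light components.
; DetectTruck overlap toggles the truck's ContainerT flag and prints an attach prompt.
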(event OnComponentBeginOverlap(DetectTruck)
  (params (OverlappedComponent :type Primitive%20Component%20Object%20Reference) (OtherActor :type Actor%20Object%20Reference) (OtherComp :type Primitive%20Component%20Object%20Reference) (OtherBodyIndex :type Integer) (bFromSweep :type Boolean) (SweepResult :type Hit%20Result%20Structure%20%28by%20ref%29))
  ;[1 1 1] DetectTruck
  (bind _astruck_bp (Utilities|Casting|CastToTruck_BP OtherActor))
  (Variables|/Game/TruckTrailer/Truck/Blueprints/Truck_BP.Truck_BP_C|SetContainerT _astruck_bp true)
  (Development|PrintString "Attach Press \"T\""))

(event OnComponentEndOverlap(DetectTruck)
  (params (OverlappedComponent :type Primitive%20Component%20Object%20Reference) (OtherActor :type Actor%20Object%20Reference) (OtherComp :type Primitive%20Component%20Object%20Reference) (OtherBodyIndex :type Integer))
  ;[1 1 1] DetectTruck
  (bind _astruck_bp (Utilities|Casting|CastToTruck_BP OtherActor))
  (Variables|/Game/TruckTrailer/Truck/Blueprints/Truck_BP.Truck_BP_C|SetContainerT _astruck_bp false))

(event EventTick
  (params (DeltaSeconds :type Float%20%28single-precision%29))
  (bind _brake (Variables|Default|GetBrake))
  (bind _side_lights (Variables|Default|GetSide_lights))
  (Utilities|FlowControl|Sequence
    (:then_0
      (if (Variables|Default|GetActive_Light)
        (Utilities|FlowControl|Sequence
          (:then_0
            ;[0.8406 0.885 0.307] Blinker
            (bind _newtrack_0 (Timeline|Timeline Play)
              (:Update
                (bind _astruck_bp (Utilities|Casting|CastToTruck_BP (Game|Player|GetPlayerPawn 0)))
                (Utilities|FlowControl|Sequence
                  (:then_0
                    (if (Variables|Default|GetF)
                      (if (Variables|/Game/TruckTrailer/Truck/Blueprints/Truck_BP.Truck_BP_C|GetLR_Blinker_Trailer _astruck_bp)
                        (Utilities|FlowControl|Sequence
                          (:then_0
                            (Rendering|Material|SetScalarParameterValue (Variables|Default|GetR_Blinker) "Light" _newtrack_0 :!class /Script/Engine.MaterialInstanceDynamic :!label _label))
                          (:then_1
                            (Rendering|Material|SetScalarParameterValue (Variables|Default|GetL_Blinker) "Light" _newtrack_0 :!class /Script/Engine.MaterialInstanceDynamic :!label _label_2)))
                        (else
                          (Utilities|FlowControl|Sequence
                            (:then_0
                              (Rendering|Material|SetScalarParameterValue (Variables|Default|GetR_Blinker) "Light" 1.0 :!class /Script/Engine.MaterialInstanceDynamic :!label _label_3))
                            (:then_1
                              (Rendering|Material|SetScalarParameterValue (Variables|Default|GetL_Blinker) "Light" 1.0 :!class /Script/Engine.MaterialInstanceDynamic :!label _label_4)))))))
                  (:then_1
                    (if (Variables|Default|GetZ)
                      (if (Variables|/Game/TruckTrailer/Truck/Blueprints/Truck_BP.Truck_BP_C|GetL_Blinker_Trailer _astruck_bp)
                        (goto _label_2)
                        (else
                          (Utilities|FlowControl|Sequence
                            (:then_0
                              (goto _label_3))
                            (:then_1
                              (goto _label_4)))))))
                  (:then_2
                    (if (Variables|Default|GetX)
                      (if (Variables|/Game/TruckTrailer/Truck/Blueprints/Truck_BP.Truck_BP_C|GetR_Blinker_Trailer _astruck_bp)
                        (goto _label)
                        (else
                          (Utilities|FlowControl|Sequence
                            (:then_0
                              (goto _label_3))
                            (:then_1
                              (goto _label_4)))))))))))
          (:then_1
            ;[1 0.653 0.5955] Side_Lights
            (bind _astruck_bp_2 (Utilities|Casting|CastToTruck_BP (Game|Player|GetPlayerPawn 0)))
            (if (Variables|/Game/TruckTrailer/Truck/Blueprints/Truck_BP.Truck_BP_C|GetActiveLightTrailer _astruck_bp_2)
              (Rendering|Material|SetScalarParameterValue _side_lights "Light" 0.0 :!class /Script/Engine.MaterialInstanceDynamic)
              (else
                (Rendering|Material|SetScalarParameterValue _side_lights "Light" 1.0 :!class /Script/Engine.MaterialInstanceDynamic :!label _label_5))))
          (:then_2
            ;[0.245 0.1151 0.1175] Brake
            (bind _astruck_bp_3 (Utilities|Casting|CastToTruck_BP (Game|Player|GetPlayerPawn 0)))
            (if (Variables|/Game/TruckTrailer/Truck/Blueprints/Truck_BP.Truck_BP_C|GetBrake_Trailer _astruck_bp_3)
              (Rendering|Material|SetVectorParameterValue _brake "Brake" (Utilities|Struct|MakeLinearColor 1e+01 0.0 0.0 0.0) :!class /Script/Engine.MaterialInstanceDynamic)
              (Rendering|Components|Light|SetIntensity (Variables|Default|GetR_Brake_Light) 1e+03)
              (elif (Variables|/Game/TruckTrailer/Truck/Blueprints/Truck_BP.Truck_BP_C|GetLight_ON_Trailer _astruck_bp_3)
                (Rendering|Material|SetVectorParameterValue (Variables|Default|GetBrake) "Brake" (Utilities|Struct|MakeLinearColor 0.5 0.0 0.0 0.0) :!class /Script/Engine.MaterialInstanceDynamic)
                (Rendering|Components|Light|SetIntensity (Variables|Default|GetR_Brake_Light) 2.5e+02)
                (else
                  (Rendering|Material|SetVectorParameterValue _brake "Brake" (Utilities|Struct|MakeLinearColor 0.0 0.0 0.0 0.0) :!class /Script/Engine.MaterialInstanceDynamic :!label _label_6)
                  (Rendering|Components|Light|SetIntensity (Variables|Default|GetR_Brake_Light) 0.0))))))
        (else
          (Utilities|FlowControl|Sequence
            (:then_0
              (goto _label_5))
            (:then_1
              (goto _label_3))
            (:then_2
              (Timeline|Timeline SetNewTime))
            (:then_3
              (goto _label_3))
            (:then_4
              (goto _label_4))
            (:then_5
              (goto _label_6))))))
    (:then_1
      ;[1 0.8889 0.5827] Control_Matching
      (bind _astruck_bp_4 (Utilities|Casting|CastToTruck_BP (Game|Player|GetPlayerPawn 0)))
      (Utilities|FlowControl|Sequence
        (:then_0
          (Variables|Default|SetF (Variables|/Game/TruckTrailer/Truck/Blueprints/Truck_BP.Truck_BP_C|GetLR_Blinker_Trailer _astruck_bp_4)))
        (:then_1
          (Variables|Default|SetZ (Variables|/Game/TruckTrailer/Truck/Blueprints/Truck_BP.Truck_BP_C|GetL_Blinker_Trailer _astruck_bp_4)))
        (:then_2
          (Variables|Default|SetX (Variables|/Game/TruckTrailer/Truck/Blueprints/Truck_BP.Truck_BP_C|GetR_Blinker_Trailer _astruck_bp_4)))))))

(fn ConstructionScript
  (bind _mesh (Variables|Character|GetMesh))
  (Utilities|FlowControl|Sequence
    (:then_0
      (bind _returnvalue (Rendering|Material|CreateDynamicMaterialInstance _mesh 1 "/Game/TruckTrailer/Trailers/ContainerTrailer/Materials/M_Brake_Box_T_Inst.M_Brake_Box_T_Inst" "None" :!class /Script/Engine.PrimitiveComponent))
      (Variables|Default|SetBrake _returnvalue))
    (:then_1
      (bind _returnvalue_2 (Rendering|Material|CreateDynamicMaterialInstance _mesh 5 "/Game/TruckTrailer/Trailers/ContainerTrailer/Materials/M_Side_light_Inst.M_Side_light_Inst" "None" :!class /Script/Engine.PrimitiveComponent))
      (Variables|Default|SetSide_lights _returnvalue_2))
    (:then_2
      (bind _returnvalue_3 (Rendering|Material|CreateDynamicMaterialInstance _mesh 6 "/Game/TruckTrailer/Trailers/ContainerTrailer/Materials/M_Box_T__Blinker_L_Inst.M_Box_T__Blinker_L_Inst" "None" :!class /Script/Engine.PrimitiveComponent))
      (Variables|Default|SetL_Blinker _returnvalue_3))
    (:then_3
      (bind _returnvalue_4 (Rendering|Material|CreateDynamicMaterialInstance _mesh 7 "/Game/TruckTrailer/Trailers/ContainerTrailer/Materials/M_Box_T__Blinker_R_Inst.M_Box_T__Blinker_R_Inst" "None" :!class /Script/Engine.PrimitiveComponent))
      (Variables|Default|SetR_Blinker _returnvalue_4))))