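; Spline-based road marking tool that builds decals or meshes along a path in the construction script.
; HeightScanner first snaps each spline point to the surface below with a visibility trace.
; Decal mode spaces a capped number of decals by scale and distance, using dynamic materials for color, quality and cracks.
; Mesh mode either stretches spline meshes over equal roughly 200-unit segments or places static meshes at set intervals.
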(fn ConstructionScript
  (bind (_return_value _returnvalue) (CallFunction|GetPathLength))
  (Utilities|FlowControl|Sequence
    (:then_0
      (|HeightScanner))
    (:then_1
      (switch Utilities|FlowControl|Switch|SwitchonENUM_ToolType (Variables|0_Settings|GetChooseType)
        (:NewEnumerator0
          (|DecalDrawer))
        (:NewEnumerator1
          (if (Variables|2_MeshDrawer|GetisStrechMesh)
            (|MeshDrawerForLines _return_value _returnvalue)
            (else
              (|MeshDrawerForDistances))))))))

(fn GetPathLength
  (bind _splinecomponent (Variables|Default|GetSplineComponent))
  (bind _returnvalue (Spline|GetSplineLength _splinecomponent))
  (bind _output_get (Variables|DoNotEdit|SetIndex (Math|Float|Truncate (/ _returnvalue 2e+02))))
  (return _output_get (/ _returnvalue (Math|Conversions|ToFloat(Integer) (Variables|DoNotEdit|GetIndex)))))