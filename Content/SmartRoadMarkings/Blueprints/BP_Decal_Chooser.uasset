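; BP_Decal_Chooser is a configurable decal actor from the SmartRoadMarkings content, displaying whichever material is assigned to DropYourMask.
; Its construction script applies sort order, fade screen size and that material to the decal component.
; It then creates a dynamic material instance and copies the actor's variables into parameters for two colors, decal quality, roughness range, three grunge layers, cracks and secondary color.
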(fn ConstructionScript
  (bind _output_get (Variables|Default|SetDecal (Variables|Default|GetDecal)))
  (Class|DecalComponent|SetSortOrder _output_get (Variables|0_DecalSettings|GetDecalOrder))
  (Rendering|Components|Decal|SetFadeScreenSize _output_get (Variables|0_DecalSettings|GetDecalFadeSize))
  (Rendering|Components|Decal|SetDecalMaterial _output_get (Variables|0_DecalSettings|GetDropYourMask))
  (bind _returnvalue (Rendering|Material|CreateDynamicMaterialInstance _output_get :!class /Script/Engine.DecalComponent))
  (Rendering|Material|SetVectorParameterValue _returnvalue "Color_A" (Variables|0_DecalSettings|GetColor_A) :!class /Script/Engine.MaterialInstanceDynamic)
  (Rendering|Material|SetVectorParameterValue _returnvalue "Color_B" (Variables|0_DecalSettings|GetColor_B) :!class /Script/Engine.MaterialInstanceDynamic)
  (Rendering|Material|SetScalarParameterValue _returnvalue "DecalQuality" (Math|Conversions|ToFloat(Integer) (Variables|0_DecalSettings|GetDecalQuality)) :!class /Script/Engine.MaterialInstanceDynamic)
  (Rendering|Material|SetScalarParameterValue _returnvalue "Roughness_Min" (Variables|4_Roughness|GetRoughness_Min) :!class /Script/Engine.MaterialInstanceDynamic)
  (Rendering|Material|SetScalarParameterValue _returnvalue "Roughness_Max" (Variables|4_Roughness|GetRoughness_Max) :!class /Script/Engine.MaterialInstanceDynamic)
  (Rendering|Material|SetScalarParameterValue _returnvalue "Grunge_1_Intensity" (Variables|3_Grunge|GetGrunge_1_Intensity) :!class /Script/Engine.MaterialInstanceDynamic)
  (Rendering|Material|SetScalarParameterValue _returnvalue "Grunge_2_Intensity" (Variables|3_Grunge|GetGrunge_2_Intensity) :!class /Script/Engine.MaterialInstanceDynamic)
  (Rendering|Material|SetScalarParameterValue _returnvalue "Grunge_3_Intensity" (Variables|3_Grunge|GetGrunge_3_Intensity) :!class /Script/Engine.MaterialInstanceDynamic)
  (Rendering|Material|SetScalarParameterValue _returnvalue "Grunge_1_Contrast" (Variables|3_Grunge|GetGrunge_1_Contrast) :!class /Script/Engine.MaterialInstanceDynamic)
  (Rendering|Material|SetScalarParameterValue _returnvalue "Grunge_2_Contrast" (Variables|3_Grunge|GetGrunge_2_Contrast) :!class /Script/Engine.MaterialInstanceDynamic)
  (Rendering|Material|SetScalarParameterValue _returnvalue "Grunge_3_Contrast" (Variables|3_Grunge|GetGrunge_3_Contrast) :!class /Script/Engine.MaterialInstanceDynamic)
  (Rendering|Material|SetScalarParameterValue _returnvalue "Grunge_1_Size" (Variables|3_Grunge|GetGrunge_1_Size) :!class /Script/Engine.MaterialInstanceDynamic)
  (Rendering|Material|SetScalarParameterValue _returnvalue "Cracks_Size" (Variables|2Cracks|GetCracks_Size) :!class /Script/Engine.MaterialInstanceDynamic)
  (Rendering|Material|SetScalarParameterValue _returnvalue "Cracks_Intensity" (Variables|2Cracks|GetCracks_Intensity) :!class /Script/Engine.MaterialInstanceDynamic)
  (Rendering|Material|SetScalarParameterValue _returnvalue "Cracks_Contrast" (Variables|2Cracks|GetCracks_Contrast) :!class /Script/Engine.MaterialInstanceDynamic)
  (Rendering|Material|SetScalarParameterValue _returnvalue "Color_Secondary_Intensity" (Variables|0_DecalSettings|GetColor_Secondary_Intensity) :!class /Script/Engine.MaterialInstanceDynamic)
  (Rendering|Material|SetScalarParameterValue _returnvalue "Color_Secondary_Size" (Variables|0_DecalSettings|GetColor_Secondary_Size) :!class /Script/Engine.MaterialInstanceDynamic))