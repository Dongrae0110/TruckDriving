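; Traffic light actor that cycles endlessly from green to yellow to red and back to green.
; BeginPlay waits a configurable delay before each change, then the Lightchange event jumps back to the first delay to repeat the loop.
; Each turn function swaps materials on the Green, Yellow and Red components, lighting one and setting the other two to an off material.
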(event Custom|Lightchange
  (Utilities|FlowControl|Delay (Variables|Default|GetGreen%20to%20Yellow))
  (CallFunction|TurnYellow)
  (Utilities|FlowControl|Delay (Variables|Default|GetYellow%20to%20Red))
  (CallFunction|TurnRed)
  (Utilities|FlowControl|Delay (Variables|Default|GetRed%20to%20Green))
  (CallFunction|TurnGreen)
  (CallFunction|Lightchange))

(event EventBeginPlay
  (Utilities|FlowControl|Delay (Variables|Default|GetGreen%20to%20Yellow))
  (CallFunction|TurnYellow)
  (Utilities|FlowControl|Delay (Variables|Default|GetYellow%20to%20Red))
  (CallFunction|TurnRed)
  (Utilities|FlowControl|Delay (Variables|Default|GetRed%20to%20Green))
  (CallFunction|TurnGreen)
  (CallFunction|Lightchange))

(event Collision|EventActorBeginOverlap
  (params (OtherActor :type Actor%20Object%20Reference)))

(event EventTick
  (params (DeltaSeconds :type Float%20%28single-precision%29)))

(fn ConstructionScript)

(fn TurnGreen
  (Rendering|Material|SetMaterial (Variables|Default|Getgreen) 0 "/Game/Traffic_light/greenmaterial1.greenmaterial1")
  (Rendering|Material|SetMaterial (Variables|Default|Getyellow) 0 "/Game/Traffic_light/lightoffmaterial.lightoffmaterial")
  (Rendering|Material|SetMaterial (Variables|Default|Getred) 0 "/Game/Traffic_light/lightoffmaterial.lightoffmaterial"))

(fn TurnYellow
  (Rendering|Material|SetMaterial (Variables|Default|Getgreen) 0 "/Game/Traffic_light/lightoffmaterial.lightoffmaterial")
  (Rendering|Material|SetMaterial (Variables|Default|Getyellow) 0 "/Game/Traffic_light/yellowmaterial2.yellowmaterial2")
  (Rendering|Material|SetMaterial (Variables|Default|Getred) 0 "/Game/Traffic_light/lightoffmaterial.lightoffmaterial"))

(fn TurnRed
  (Rendering|Material|SetMaterial (Variables|Default|Getgreen) 0 "/Game/Traffic_light/lightoffmaterial.lightoffmaterial")
  (Rendering|Material|SetMaterial (Variables|Default|Getyellow) 0 "/Game/Traffic_light/lightoffmaterial.lightoffmaterial")
  (Rendering|Material|SetMaterial (Variables|Default|Getred) 0 "/Game/Traffic_light/redmaterial.redmaterial"))